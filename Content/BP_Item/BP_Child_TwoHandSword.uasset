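; Two-handed sword item, a child Blueprint that switches the player character (Jack) to this weapon when used.
; The construction script fills its stat structs from per-topic data tables, covering item, damage, movement, stamina, block/parry, range, sound and HUD, in a nested chain where one missing row skips the rest.
; BeginPlay sets durability, UseItem passes the weapon multiplier to ChangeWeapon, and DoStaff only prints a string.
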(event `self.ReceiveBeginPlay`
  (`parent.ReceiveBeginPlay`)
  (`self.SetDurability`))

(event `self.DoStaff`
  (`KismetSystemLibrary.PrintString` "give us health"))

(fn `UseItem`
  (returns (Success :type Boolean))
  (bind _success (`parent.UseItem`))
  (`/Game/SideScrollerBP/Blueprints/PC_Jack.ChangeWeapon` (`self.PCJack`) "BP_Child_TwoHandSword_C" (`.WeaponMultiply_2_A794AEC04CF257BB7F606391A760184B` (break `/Game/Structure_Data/Jack/DamageSystem/S_WeaponMultply` (`self.PIWeaponMultiply`))) self)
  (return _success))

(fn `UserConstructionScript`
  (`parent.UserConstructionScript`)
  (bind _returnvalue (`|GetDataTableRow` "/Game/Structure_Data/DataItemStats.DataItemStats" "TwoHandedSword01")
    (:`then`
      (set `self.ParentItemData` _returnvalue)
      (bind _returnvalue_2 (`|GetDataTableRow` "/Game/Structure_Data/Jack/DamageSystem/Data_WeaponMultiply.Data_WeaponMultiply" "TwoHandedSword01")
        (:`then`
          (set `self.PIWeaponMultiply` _returnvalue_2)
          (bind _returnvalue_3 (`|GetDataTableRow` "/Game/Structure_Data/Jack/DamageSystem/Data_JackAttackTypeMultiply.Data_JackAttackTypeMultiply" "TwoHandSword01")
            (:`then`
              (set `self.PI_AttackTypeMultiply` _returnvalue_3)
              (bind _returnvalue_4 (`|GetDataTableRow` "/Game/Structure_Data/Item/Data_SocketName.Data_SocketName" "TwoHandSword01")
                (:`then`
                  (set `self.PI_SocketName` _returnvalue_4)
                  (bind _returnvalue_5 (`|GetDataTableRow` "/Game/Structure_Data/Item/Data_WeaponTypeMovement.Data_WeaponTypeMovement" "TwoHanded01")
                    (:`then`
                      (set `self.PI_WeaponTypeMovement` _returnvalue_5)
                      (bind _returnvalue_6 (`|GetDataTableRow` "/Game/Structure_Data/Item/Data_WeaponTypeAttack.Data_WeaponTypeAttack" "TwoHandSword01")
                        (:`then`
                          (set `self.PI_WeaponTypeAttack` _returnvalue_6)
                          (bind _returnvalue_7 (`|GetDataTableRow` "/Game/Structure_Data/Jack/StaminaSystem/Data_WeaponTypeStamina.Data_WeaponTypeStamina" "TwoHandSword01")
                            (:`then`
                              (set `self.PI_WeaponTypeStamina` _returnvalue_7)
                              (bind _returnvalue_8 (`|GetDataTableRow` "/Game/Structure_Data/Item/Data_BlockWeaponType.Data_BlockWeaponType" "TwoHandedSword")
                                (:`then`
                                  (set `self.PI_BlockWeaponType` _returnvalue_8)
                                  (bind _returnvalue_9 (`|GetDataTableRow` "/Game/Structure_Data/Item/D_BlockParryMultiply_WT.D_BlockParryMultiply_WT" "TwoHandSword01")
                                    (:`then`
                                      (set `self.PI_BlockParryMultiply_WT` _returnvalue_9)
                                      (bind _returnvalue_10 (`|GetDataTableRow` "/Game/Structure_Data/Item/Data_AttackRangeWeaponType.Data_AttackRangeWeaponType" "TwoHandSword01")
                                        (:`then`
                                          (set `self.PI_AttackRange_WT` _returnvalue_10)
                                          (bind _returnvalue_11 (`|GetDataTableRow` "/Game/Structure_Data/Item/D_SoundWeaponType.D_SoundWeaponType" "TwoHandedWord1")
                                            (:`then`
                                              (set `self.PI_Sound_WT` _returnvalue_11)
                                              (bind _returnvalue_12 (`|GetDataTableRow` "/Game/Structure_Data/Item/D_WeaponHUD.D_WeaponHUD" "TwoHandedSword01")
                                                (:`then`
                                                  (set `self.PI_WeaponHUD` _returnvalue_12)
                                                  (bind _returnvalue_13 (`|GetDataTableRow` "/Game/Structure_Data/Item/D_AttackTypeDamageToWeapon.D_AttackTypeDamageToWeapon" "TwoHandedSword01")
                                                    (:`then`
                                                      (set `self.PI_AttackTypeDamageToWeapon` _returnvalue_13))))))))))))))))))))))))))))