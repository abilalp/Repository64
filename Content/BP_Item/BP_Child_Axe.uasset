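; BP_Child_Axe is the axe weapon item, a child Blueprint that equips itself on the player.
; Its construction script fills item stats and weapon-type data (multipliers, socket, movement, attack, stamina, block/parry, range, sound) through chained data table lookups, each dependent on the previous row being found.
; Rows are keyed "Axe01", except attack, which reads "Sword01", and sound, which reads "Axe1".
; UseItem calls the parent, then PCJack's ChangeWeapon with the weapon multiplier.
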(fn `UseItem`
  (returns (Success :type Boolean))
  (bind _success (`parent.UseItem`))
  (`/Game/SideScrollerBP/Blueprints/PC_Jack.ChangeWeapon` (`self.PCJack`) "BP_Child_Axe_C" (`.WeaponMultiply_2_A794AEC04CF257BB7F606391A760184B` (break `/Game/Structure_Data/Jack/DamageSystem/S_WeaponMultply` (`self.PIWeaponMultiply`))) self)
  (return _success))

(fn `UserConstructionScript`
  (`parent.UserConstructionScript`)
  (bind _returnvalue (`|GetDataTableRow` "/Game/Structure_Data/DataItemStats.DataItemStats" "Axe01")
    (:`then`
      (set `self.ParentItemData` _returnvalue)
      (bind _returnvalue_2 (`|GetDataTableRow` "/Game/Structure_Data/Jack/DamageSystem/Data_WeaponMultiply.Data_WeaponMultiply" "Axe01")
        (:`then`
          (set `self.PIWeaponMultiply` _returnvalue_2)
          (bind _returnvalue_3 (`|GetDataTableRow` "/Game/Structure_Data/Jack/DamageSystem/Data_JackAttackTypeMultiply.Data_JackAttackTypeMultiply" "Axe01")
            (:`then`
              (set `self.PI_AttackTypeMultiply` _returnvalue_3)
              (bind _returnvalue_4 (`|GetDataTableRow` "/Game/Structure_Data/Item/Data_SocketName.Data_SocketName" "Axe01")
                (:`then`
                  (set `self.PI_SocketName` _returnvalue_4)
                  (bind _returnvalue_5 (`|GetDataTableRow` "/Game/Structure_Data/Item/Data_WeaponTypeMovement.Data_WeaponTypeMovement" "Axe01")
                    (:`then`
                      (set `self.PI_WeaponTypeMovement` _returnvalue_5)
                      (bind _returnvalue_6 (`|GetDataTableRow` "/Game/Structure_Data/Item/Data_WeaponTypeAttack.Data_WeaponTypeAttack" "Sword01")
                        (:`then`
                          (set `self.PI_WeaponTypeAttack` _returnvalue_6)
                          (bind _returnvalue_7 (`|GetDataTableRow` "/Game/Structure_Data/Jack/StaminaSystem/Data_WeaponTypeStamina.Data_WeaponTypeStamina" "Axe01")
                            (:`then`
                              (set `self.PI_WeaponTypeStamina` _returnvalue_7)
                              (bind _returnvalue_8 (`|GetDataTableRow` "/Game/Structure_Data/Item/Data_BlockWeaponType.Data_BlockWeaponType" "Axe01")
                                (:`then`
                                  (set `self.PI_BlockWeaponType` _returnvalue_8)
                                  (bind _returnvalue_9 (`|GetDataTableRow` "/Game/Structure_Data/Item/D_BlockParryMultiply_WT.D_BlockParryMultiply_WT" "Axe01")
                                    (:`then`
                                      (set `self.PI_BlockParryMultiply_WT` _returnvalue_9)
                                      (bind _returnvalue_10 (`|GetDataTableRow` "/Game/Structure_Data/Item/Data_AttackRangeWeaponType.Data_AttackRangeWeaponType" "Axe01")
                                        (:`then`
                                          (set `self.PI_AttackRange_WT` _returnvalue_10)
                                          (bind _returnvalue_11 (`|GetDataTableRow` "/Game/Structure_Data/Item/D_SoundWeaponType.D_SoundWeaponType" "Axe1")
                                            (:`then`
                                              (set `self.PI_Sound_WT` _returnvalue_11))))))))))))))))))))))))