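; BP_Child_Spear is the spear weapon item, a child Blueprint that equips itself on the Jack character when used.
; Its construction script fills inherited weapon stats from chained data table lookups on row Spear01, covering multipliers, socket, movement, attack, stamina, block/parry and range.
; The attack-type multiplier reads row Sword01 instead, and any missing row stops the remaining lookups.
; UseItem runs the parent logic, then passes itself and its weapon multiplier to PCJack's ChangeWeapon.
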(fn `UseItem`
  (returns (Success :type Boolean))
  (bind _success (`parent.UseItem`))
  (`/Game/SideScrollerBP/Blueprints/PC_Jack.ChangeWeapon` (`self.PCJack`) "BP_Child_Spear_C" (`.WeaponMultiply_2_A794AEC04CF257BB7F606391A760184B` (break `/Game/Structure_Data/Jack/DamageSystem/S_WeaponMultply` (`self.PIWeaponMultiply`))) self)
  (return _success))

(fn `UserConstructionScript`
  (`parent.UserConstructionScript`)
  (bind _returnvalue (`|GetDataTableRow` "/Game/Structure_Data/Jack/DamageSystem/Data_WeaponMultiply.Data_WeaponMultiply" "Spear01")
    (:`then`
      (set `self.PIWeaponMultiply` _returnvalue)
      (bind _returnvalue_2 (`|GetDataTableRow` "/Game/Structure_Data/Jack/DamageSystem/Data_JackAttackTypeMultiply.Data_JackAttackTypeMultiply" "Sword01")
        (:`then`
          (set `self.PI_AttackTypeMultiply` _returnvalue_2)
          (bind _returnvalue_3 (`|GetDataTableRow` "/Game/Structure_Data/Item/Data_SocketName.Data_SocketName" "Spear01")
            (:`then`
              (set `self.PI_SocketName` _returnvalue_3)
              (bind _returnvalue_4 (`|GetDataTableRow` "/Game/Structure_Data/Item/Data_WeaponTypeMovement.Data_WeaponTypeMovement" "Spear01")
                (:`then`
                  (set `self.PI_WeaponTypeMovement` _returnvalue_4)
                  (bind _returnvalue_5 (`|GetDataTableRow` "/Game/Structure_Data/Item/Data_WeaponTypeAttack.Data_WeaponTypeAttack" "Spear01")
                    (:`then`
                      (set `self.PI_WeaponTypeAttack` _returnvalue_5)
                      (bind _returnvalue_6 (`|GetDataTableRow` "/Game/Structure_Data/Jack/StaminaSystem/Data_WeaponTypeStamina.Data_WeaponTypeStamina" "Spear01")
                        (:`then`
                          (set `self.PI_WeaponTypeStamina` _returnvalue_6)
                          (bind _returnvalue_7 (`|GetDataTableRow` "/Game/Structure_Data/Item/Data_BlockWeaponType.Data_BlockWeaponType" "Spear01")
                            (:`then`
                              (set `self.PI_BlockWeaponType` _returnvalue_7)
                              (bind _returnvalue_8 (`|GetDataTableRow` "/Game/Structure_Data/Item/D_BlockParryMultiply_WT.D_BlockParryMultiply_WT" "Spear01")
                                (:`then`
                                  (set `self.PI_BlockParryMultiply_WT` _returnvalue_8)
                                  (bind _returnvalue_9 (`|GetDataTableRow` "/Game/Structure_Data/Item/Data_AttackRangeWeaponType.Data_AttackRangeWeaponType" "Spear01")
                                    (:`then`
                                      (set `self.PI_AttackRange_WT` _returnvalue_9))))))))))))))))))))