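; Base item/weapon actor for the side-scroller that Jack can pick up and that wears out with use.
; The Construction Script fills stat, multiplier, socket, movement, attack, block, sound and HUD structs through chained data table lookups.
; Interact hands it to PC_Jack's inventory if space allows, then hides it and disables collision.
; Attack-type events subtract durability from its data-driven maximum, while Tick polls for zero and calls PC_Jack's DestroyWeapon.
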(event `self.ReceiveBeginPlay`
  ;[1 1 1] Get ref
  (bind _asside_scroller_character (cast `/Game/SideScrollerBP/Blueprints/SideScrollerCharacter` (`GameplayStatics.GetPlayerCharacter` 0)))
  (set `self.Jack` _asside_scroller_character)
  (bind _aspc_jack (cast `/Game/SideScrollerBP/Blueprints/PC_Jack` (`GameplayStatics.GetPlayerController` 0)))
  (set `self.PCJack` _aspc_jack)
  (`self.SetDurability`))

(event `self.ReceiveTick`
  (params (DeltaSeconds :type "Float (single-precision)"))
  ;[1 1 1] if weapon durability is below 0, weapon will destroy. the code is written in the jack PC
  (if (<= (`self.WeaponDurability`) 0.0)
    (`/Game/SideScrollerBP/Blueprints/PC_Jack.DestroyWeapon` (`self.PCJack`))))

(event `/Game/BPI/BPI_InteractItem.Interact`
  (params (InteracterController :type "/Game/SideScrollerBP/Blueprints/PC_Jack Object Reference") (Success :type Boolean))
  (bind _pcjack (`self.PCJack`))
  ;[1 1 1] Pick Up Item If has space
  (bind _hasspace_ (`/Game/SideScrollerBP/Blueprints/PC_Jack.InventoryCheck` (`self.PCJack`)))
  (if _hasspace_
    (`/Game/SideScrollerBP/Blueprints/PC_Jack.Pickup Item` _pcjack self (`/Game/SideScrollerBP/Blueprints/PC_Jack.InventoryObjects` _pcjack))
    (`self.SetActorHiddenInGame` true)
    (`self.SetActorEnableCollision` false)
    (else
      (`KismetSystemLibrary.PrintString` "InventoryFull"))))

(event `DoStaff`
  (`KismetSystemLibrary.PrintString` "Do coll stuff"))

(event `/Game/BPI/BPI_InteractItem.ToWeaponLeftDamage1`
  (`self.UpdateWeaponDurability` (`.Left1_4_4AA6086E42664F92C6B4C08EE63869DE` (break `/Game/Structure_Data/Item/S_AttackTypeDamageToWeapon` (`self.PI_AttackTypeDamageToWeapon`)))))

(event `/Game/BPI/BPI_InteractItem.ToWeaponLeftDamage2`
  (`self.UpdateWeaponDurability` (`.left2_5_3C4208884F3B9C79B77B64B3E579FE84` (break `/Game/Structure_Data/Item/S_AttackTypeDamageToWeapon` (`self.PI_AttackTypeDamageToWeapon`)))))

(event `/Game/BPI/BPI_InteractItem.ToWeaponRightDamage1`
  (`self.UpdateWeaponDurability` (`.Right1_7_8984D5BE48B81D7534E8AFBFD080BE58` (break `/Game/Structure_Data/Item/S_AttackTypeDamageToWeapon` (`self.PI_AttackTypeDamageToWeapon`)))))

(event `/Game/BPI/BPI_InteractItem.ToWeaponRightDamage2`
  (`self.UpdateWeaponDurability` (`.Right2_9_86E579224FC211E72D7C54BAAE9B0E65` (break `/Game/Structure_Data/Item/S_AttackTypeDamageToWeapon` (`self.PI_AttackTypeDamageToWeapon`)))))

(event `/Game/BPI/BPI_InteractItem.ToWeaponUpperDamage`
  (`self.UpdateWeaponDurability` (`.Upper_11_7AA7613C462B3A531B271DB5E71D6922` (break `/Game/Structure_Data/Item/S_AttackTypeDamageToWeapon` (`self.PI_AttackTypeDamageToWeapon`)))))

(fn `ChangeSphereCollision`
  (bind _trigger (`self.Trigger`))
  (`PrimitiveComponent.SetCollisionResponseToAllChannels` _trigger "ECR_Ignore")
  (`PrimitiveComponent.SetCollisionEnabled` _trigger "NoCollision"))

(fn `SetDurability`
  (set `self.WeaponDurability` (`.DurabilityMax_4_E422DDBB45A5429B486C39B46A3C332C` (break `/Game/Structure_Data/Item/S_WeaponHUD` (`self.PI_WeaponHUD`))))
  (return))

(fn `UseItem`
  (returns (Success :type Boolean))
  (return true))

(fn `UserConstructionScript`
  (bind _returnvalue (`|GetDataTableRow` "/Game/Structure_Data/DataItemStats.DataItemStats" "PatentItem")
    (:`then`
      (set `self.ParentItemData` _returnvalue)
      (bind _returnvalue_2 (`|GetDataTableRow` "/Game/Structure_Data/Jack/DamageSystem/Data_WeaponMultiply.Data_WeaponMultiply" "ParentItem")
        (:`then`
          (set `self.PIWeaponMultiply` _returnvalue_2)
          (bind _returnvalue_3 (`|GetDataTableRow` "/Game/Structure_Data/Jack/DamageSystem/Data_JackAttackTypeMultiply.Data_JackAttackTypeMultiply" "ParentWeapon")
            (:`then`
              (set `self.PI_AttackTypeMultiply` _returnvalue_3)
              (bind _returnvalue_4 (`|GetDataTableRow` "/Game/Structure_Data/Item/Data_SocketName.Data_SocketName" "ParentItem")
                (:`then`
                  (set `self.PI_SocketName` _returnvalue_4)
                  (bind _returnvalue_5 (`|GetDataTableRow` "/Game/Structure_Data/Item/Data_WeaponTypeMovement.Data_WeaponTypeMovement" "ParentItem")
                    (:`then`
                      (set `self.PI_WeaponTypeMovement` _returnvalue_5)
                      (bind _returnvalue_6 (`|GetDataTableRow` "/Game/Structure_Data/Item/Data_WeaponTypeAttack.Data_WeaponTypeAttack" "ParentItem")
                        (:`then`
                          (set `self.PI_WeaponTypeAttack` _returnvalue_6)
                          (bind _returnvalue_7 (`|GetDataTableRow` "/Game/Structure_Data/Jack/StaminaSystem/Data_WeaponTypeStamina.Data_WeaponTypeStamina" "ParentItem")
                            (:`then`
                              (set `self.PI_WeaponTypeStamina` _returnvalue_7)
                              (bind _returnvalue_8 (`|GetDataTableRow` "/Game/Structure_Data/Item/Data_BlockWeaponType.Data_BlockWeaponType" "ParentItem")
                                (:`then`
                                  (set `self.PI_BlockWeaponType` _returnvalue_8)
                                  (bind _returnvalue_9 (`|GetDataTableRow` "/Game/Structure_Data/Item/D_BlockParryMultiply_WT.D_BlockParryMultiply_WT" "ParentItem")
                                    (:`then`
                                      (set `self.PI_BlockParryMultiply_WT` _returnvalue_9)
                                      (bind _returnvalue_10 (`|GetDataTableRow` "/Game/Structure_Data/Item/Data_AttackRangeWeaponType.Data_AttackRangeWeaponType" "EnemyItem")
                                        (:`then`
                                          (set `self.PI_AttackRange_WT` _returnvalue_10)
                                          (bind _returnvalue_11 (`|GetDataTableRow` "/Game/Structure_Data/Item/D_SoundWeaponType.D_SoundWeaponType" "ParentItem")
                                            (:`then`
                                              (set `self.PI_Sound_WT` _returnvalue_11)
                                              (bind _returnvalue_12 (`|GetDataTableRow` "/Game/Structure_Data/Item/D_WeaponHUD.D_WeaponHUD" "ParentItem")
                                                (:`then`
                                                  (set `self.PI_WeaponHUD` _returnvalue_12)
                                                  (bind _returnvalue_13 (`|GetDataTableRow` "/Game/Structure_Data/Item/D_AttackTypeDamageToWeapon.D_AttackTypeDamageToWeapon" "ParentItem")
                                                    (:`then`
                                                      (set `self.PI_AttackTypeDamageToWeapon` _returnvalue_13))))))))))))))))))))))))))))