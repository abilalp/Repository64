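; Demon fire projectile actor that launches forward and slightly downward on BeginPlay and explodes on overlap.
; The construction script configures Niagara effects, movement and rotation, and loads the "Fireball02" damage row when the projectile VFX is valid.
; Box overlap spawns an explosion, sends hit-reaction and damage messages if it hits Jack (SideScrollerCharacter), then destroys the projectile.
; Overlaps with any other actor only explode and destroy it.
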(event `self.ReceiveBeginPlay`
  (`ProjectileMovementComponent.SetVelocityInLocalSpace` (`self.ProjectileMovement`) (2000.0 0.0 -250.0)))

(event `self.BoxCollision.OnComponentBeginOverlap`
  (params (OverlappedComponent :type "PrimitiveComponent Object Reference") (OtherActor :type "Actor Object Reference") (OtherComp :type "PrimitiveComponent Object Reference") (OtherBodyIndex :type Integer) (bFromSweep :type Boolean) (SweepResult :type "HitResult Structure (by ref)"))
  (bind _jack (`self.Jack`))
  (set `self.ProjectileOverlapJack` false)
  (`KismetArrayLibrary.Array_Clear` (`self.Jacks`))
  (bind _asside_scroller_character (cast `/Game/SideScrollerBP/Blueprints/SideScrollerCharacter` OtherActor)
    (:`then`
      (set `self.Jack` _asside_scroller_character)
      (if (not (`KismetArrayLibrary.Array_Contains` (`self.Jacks`) (`self.Jack`)))
        (`KismetArrayLibrary.Array_Add` (`self.Jacks`) (`self.Jack`))
        (`NiagaraFunctionLibrary.SpawnSystemAtLocation` "/Game/VFX/Fireball14/Explosion/NS_Explosion.NS_Explosion" (+ (`SceneComponent.K2_GetComponentLocation` (`self.BoxCollision`)) (0.0 0.0 0.0)) (struct) (2.0 2.0 2.0))
        (set `self.ProjectileOverlapJack` true)
        (message `/Game/BPI/BPI_JackEnemyCombat.JackHitReactionFireballFront` _jack self self (`self.ProjectileOverlapJack`))
        (message `/Game/BPI/BPI_JackEnemyCombat.ProjectileDamageAmount` _jack)
        (`self.AfterCollideDestroyActor`)
        (`KismetArrayLibrary.Array_Clear` (`self.Jacks`))
        (`KismetSystemLibrary.Delay` 0.1)
        (set `self.Jack` null)))
    (:`CastFailed`
      (`self.SearchStaticMesh`))))

(event `SearchStaticMesh`
  (bind _boxcollision (`self.BoxCollision`))
  (bind (_returnvalue_location _returnvalue_rotation) (`KismetMathLibrary.BreakTransform` (`SceneComponent.K2_GetComponentToWorld` _boxcollision)))
  (`NiagaraFunctionLibrary.SpawnSystemAtLocation` "/Game/VFX/Fireball14/Explosion/NS_Explosion.NS_Explosion" (+ (`SceneComponent.K2_GetComponentLocation` _boxcollision) (20.0 0.0 0.0)) _returnvalue_rotation)
  (`self.AfterCollideDestroyActor`))

(fn `UserConstructionScript`
  (bind _scale (`self.Scale`))
  (bind _projectileniagara (`self.ProjectileNiagara`))
  (if (`KismetSystemLibrary.IsValid` (`self.VFXProjectile Niagara`))
    (`NiagaraComponent.SetAsset` (`self.ProjectileNiagara`) (`self.VFXProjectile Niagara`))
    (`NiagaraComponent.SetAsset` (`self.HitNiagara`) (`self.VFXHit Niagara`))
    (`NiagaraComponent.SetAsset` (`self.MuzzleNiagara`) (`self.VFXMuzzle Niagara`))
    (set `ProjectileMovementComponent.InitialSpeed` (`self.Projectile Speed`) (`self.ProjectileMovement`))
    (`ActorComponent.SetAutoActivate` (`self.HitNiagara`) false)
    (`ActorComponent.SetAutoActivate` (`self.MuzzleNiagara`) false)
    (`ActorComponent.SetAutoActivate` (`self.ProjectileNiagara`) false)
    (set `RotatingMovementComponent.RotationRate` (`self.Rotation Rate`) (`self.RotatingMovement`))
    (`NiagaraComponent.SetVariableVec3` _projectileniagara "Scale" _scale)
    (`NiagaraComponent.SetVariableVec3` (`self.HitNiagara`) "Scale" _scale)
    (`NiagaraComponent.SetVariableVec3` (`self.MuzzleNiagara`) "Scale" _scale)
    (`NiagaraComponent.SetVariableFloat` _projectileniagara "Scale" (.x _scale))
    (`NiagaraComponent.SetVariableFloat` (`self.HitNiagara`) "Scale" (.x _scale))
    (`NiagaraComponent.SetVariableFloat` (`self.MuzzleNiagara`) "Scale" (.x _scale))
    (bind _returnvalue (`|GetDataTableRow` "/Game/Structure_Data/Jack/Data_JackDamageAmount.Data_JackDamageAmount" "Fireball02")
      (:`then`
        (set `self.D_JackFireballDamage` _returnvalue)))))