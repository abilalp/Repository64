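; Jack's fire projectile, which launches forward and slightly upward on spawn and explodes on overlap.
; The construction script applies configurable projectile, hit and muzzle Niagara assets, scale, speed and rotation rate, with auto-activation off.
; An overlapped Bp_ParentEnemy receives hit-reaction and damage messages, while any other actor just triggers the explosion.
; Both paths spawn NS_Explosion, then stop and destroy the projectile.
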(event `self.ReceiveBeginPlay`
  (`ProjectileMovementComponent.SetVelocityInLocalSpace` (`self.ProjectileMovement`) (1000.0 0.0 200.0)))

(event `self.BoxCollision.OnComponentBeginOverlap`
  (params (OverlappedComponent :type "PrimitiveComponent Object Reference") (OtherActor :type "Actor Object Reference") (OtherComp :type "PrimitiveComponent Object Reference") (OtherBodyIndex :type Integer) (bFromSweep :type Boolean) (SweepResult :type "HitResult Structure (by ref)"))
  (bind _damagetarget (`self.DamageTarget`))
  (`KismetArrayLibrary.Array_Clear` (`self.DamageTargets`))
  (bind _asbp_parent_enemy (cast `/Game/Ai/ParentEnemy/Bp_ParentEnemy` OtherActor)
    (:`then`
      (set `self.DamageTarget` _asbp_parent_enemy)
      (if (not (`KismetArrayLibrary.Array_Contains` (`self.DamageTargets`) (`self.DamageTarget`)))
        (`KismetArrayLibrary.Array_Add` (`self.DamageTargets`) (`self.DamageTarget`))
        (`NiagaraFunctionLibrary.SpawnSystemAtLocation` "/Game/VFX/Fireball14/Explosion/NS_Explosion.NS_Explosion" (+ (`SceneComponent.K2_GetComponentLocation` (`self.BoxCollision`)) (0.0 -55.0 0.0)) (struct) (2.0 2.0 2.0))
        (message `/Game/BPI/BPI_JackEnemyCombat.EnemyHitReactionUpperAttack` _damagetarget self (0.0 0.0 0.0))
        (message `/Game/BPI/BPI_JackEnemyCombat.ProjectileDamageAmount` _damagetarget)
        (`self.AfterCollideDestroyActor`)
        (`KismetArrayLibrary.Array_Clear` (`self.DamageTargets`))
        (`KismetSystemLibrary.Delay` 0.1)
        (set `self.DamageTarget` null)))
    (:`CastFailed`
      (`self.jackSearchStaticMesh`))))

(event `JackSearchStaticMesh`
  (bind _boxcollision (`self.BoxCollision`))
  (bind (_returnvalue_location _returnvalue_rotation) (`KismetMathLibrary.BreakTransform` (`SceneComponent.K2_GetComponentToWorld` _boxcollision)))
  (`NiagaraFunctionLibrary.SpawnSystemAtLocation` "/Game/VFX/Fireball14/Explosion/NS_Explosion.NS_Explosion" (+ (`SceneComponent.K2_GetComponentLocation` _boxcollision) (100.0 0.0 0.0)) _returnvalue_rotation)
  (`self.AfterCollideDestroyActor`))

(fn `UserConstructionScript`
  (bind _scale (`self.Scale`))
  (bind _projectileniagara (`self.ProjectileNiagara`))
  (if (`KismetSystemLibrary.IsValid` (`self.VFXProjectile Niagara`))
    (`NiagaraComponent.SetAsset` (`self.ProjectileNiagara`) (`self.VFXProjectile Niagara`))
    (`NiagaraComponent.SetAsset` (`self.HitNiagara`) (`self.VFXHit Niagara`))
    (`NiagaraComponent.SetAsset` (`self.MuzzleNiagara`) (`self.VFXMuzzle Niagara`))
    (set `ProjectileMovementComponent.InitialSpeed` (`self.Projectile Speed`) (`self.ProjectileMovement`))
    (`ActorComponent.SetAutoActivate` (`self.HitNiagara`) false)
    (`ActorComponent.SetAutoActivate` (`self.MuzzleNiagara`) false)
    (`ActorComponent.SetAutoActivate` (`self.ProjectileNiagara`) false)
    (set `RotatingMovementComponent.RotationRate` (`self.Rotation Rate`) (`self.RotatingMovement`))
    (`NiagaraComponent.SetVariableVec3` _projectileniagara "Scale" _scale)
    (`NiagaraComponent.SetVariableVec3` (`self.HitNiagara`) "Scale" _scale)
    (`NiagaraComponent.SetVariableVec3` (`self.MuzzleNiagara`) "Scale" _scale)
    (`NiagaraComponent.SetVariableFloat` _projectileniagara "Scale" (.x _scale))
    (`NiagaraComponent.SetVariableFloat` (`self.HitNiagara`) "Scale" (.x _scale))
    (`NiagaraComponent.SetVariableFloat` (`self.MuzzleNiagara`) "Scale" (.x _scale))))